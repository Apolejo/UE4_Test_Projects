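; Traffic light actor that cycles red, yellow, green and yellow on timed delays and applies its state to an overlapping BP_MyVehicle.
; A recursive SetLight event started at BeginPlay swaps the mesh material and calls SetVehicleMovement with the color index.
; On trigger entry it also reroutes the vehicle, from MainPath to a random spline in MySplines or from any other spline back to MainPath.
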(event OnComponentBeginOverlap(TrafficLightCollision)
  (params (OverlappedComponent :type Primitive%20Component%20Object%20Reference) (OtherActor :type Actor%20Object%20Reference) (OtherComp :type Primitive%20Component%20Object%20Reference) (OtherBodyIndex :type Integer) (bFromSweep :type Boolean) (SweepResult :type Hit%20Result%20Structure%20%28by%20ref%29))
  (bind _mysplines (Variables|Default|GetMySplines))
  (bind _mainpath (Variables|TrafficLight|GetMainPath))
  (bind _asbp_my_vehicle (Utilities|Casting|CastToBP_MyVehicle OtherActor))
  (Variables|Default|SetVehicle_Ref _asbp_my_vehicle)
  (Class|TrafficLight|SetVehicleMovement (Variables|Default|GetColor_Index))
  (Variables|Default|SetControl_Index (Math|Random|RandomInteger (Utilities|Array|Length _mysplines)))
  (Utilities|IsValid (Utilities|Array|Get(acopy) _mysplines (Variables|Default|GetControl_Index))
    (:Is%20Valid
      (if (== (Variables|/Script/SaberPorto_Test.MySaberPorto_MyVehicle|GetCurrentSpline _asbp_my_vehicle) _mainpath)
        (Class|WheeledVehicleMovementComponent|SetThrottleInput (Variables|/Script/PhysXVehicles.WheeledVehicle|GetVehicleMovement _asbp_my_vehicle) 0.0)
        (Variables|/Script/SaberPorto_Test.SplinePathActor|SetActorToMove (Variables|/Script/SaberPorto_Test.MySaberPorto_MyVehicle|GetCurrentSpline _asbp_my_vehicle) 0)
        (Variables|/Script/SaberPorto_Test.MySaberPorto_MyVehicle|SetCurrentSpline (Variables|Default|GetVehicle_Ref) (Utilities|Array|Get(acopy) _mysplines (Variables|Default|GetControl_Index)))
        (Class|SplinePathActor|ReplaceReference (Utilities|Array|Get(acopy) _mysplines (Variables|Default|GetControl_Index)) (Variables|Default|GetVehicle_Ref))
        (else
          (Variables|/Script/SaberPorto_Test.SplinePathActor|SetActorToMove (Variables|/Script/SaberPorto_Test.MySaberPorto_MyVehicle|GetCurrentSpline _asbp_my_vehicle) 0)
          (Variables|/Script/SaberPorto_Test.MySaberPorto_MyVehicle|SetCurrentSpline (Variables|Default|GetVehicle_Ref) _mainpath)
          (Class|SplinePathActor|ReplaceReference _mainpath (Variables|Default|GetVehicle_Ref)))))))

(event OnComponentEndOverlap(TrafficLightCollision)
  (params (OverlappedComponent :type Primitive%20Component%20Object%20Reference) (OtherActor :type Actor%20Object%20Reference) (OtherComp :type Primitive%20Component%20Object%20Reference) (OtherBodyIndex :type Integer))
  (Utilities|Casting|CastToBP_MyVehicle OtherActor)
  (Variables|Default|SetVehicle_Ref 0))

(event Custom|SetLight
  (bind _trafficlightmesh (Variables|Default|GetTrafficLightMesh))
  (Variables|Default|GetVehicle_Ref
    (:then
      (Class|TrafficLight|SetVehicleMovement (Variables|Default|GetColor_Index)))
    (:else
      _))
  (switch int (Variables|Default|GetColor_Index)
    (:0
      (Rendering|Material|SetMaterial _trafficlightmesh 0 "/Game/Geometry/Meshes/RedLight_Material.RedLight_Material")
      (Utilities|FlowControl|Delay 6.0 :!label _label)
      (Math|Integer|IncrementInt (Variables|Default|GetColor_Index)
        (:%20%20
          (CallFunction|SetLight))))
    (:1
      (Rendering|Material|SetMaterial _trafficlightmesh 0 "/Game/Geometry/Meshes/YellowLight_Material.YellowLight_Material")
      (goto _label))
    (:2
      (Rendering|Material|SetMaterial _trafficlightmesh 0 "/Game/Geometry/Meshes/GreenLight_Material.GreenLight_Material")
      (goto _label))
    (:3
      (Rendering|Material|SetMaterial _trafficlightmesh 0 "/Game/Geometry/Meshes/YellowLight_Material.YellowLight_Material")
      (Utilities|FlowControl|Delay 3.0)
      (Variables|Default|SetColor_Index 0)
      (CallFunction|SetLight))))

(event EventBeginPlay
  (CallFunction|SetLight))

(event Collision|EventActorBeginOverlap
  (params (OtherActor :type Actor%20Object%20Reference)))

(event EventTick
  (params (DeltaSeconds :type Float%20%28single-precision%29)))

(fn ConstructionScript)