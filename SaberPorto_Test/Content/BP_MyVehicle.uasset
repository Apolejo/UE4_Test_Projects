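; BP_MyVehicle is a vehicle Blueprint that drives its own stats HUD.
; On BeginPlay it creates a WBP_Stats widget, keeps a reference and adds it to the viewport.
; Every Tick it pushes the speed display string and gas progress into the widget.
; The UpdateUI_Score event adds 10 to the score through AddScore and writes the result to the widget.
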(event Custom|UpdateUI_Score
  (bind _returnvalue (Class|MySaberPortoMyVehicle|AddScore 10))
  (Variables|/Game/UMG/WBP_Stats.WBP_Stats_C|SetScore (Variables|Default|GetWBP_Stats_Ref) _returnvalue))

(event EventBeginPlay
  (bind _returnvalue (UserInterface|CreateWidget "/Game/UMG/WBP_Stats.WBP_Stats_C"))
  (Variables|Default|SetWBP_Stats_Ref _returnvalue)
  (UserInterface|Viewport|AddtoViewport _returnvalue 0))

(event Collision|EventActorBeginOverlap
  (params (OtherActor :type Actor%20Object%20Reference)))

(event EventTick
  (params (DeltaSeconds :type Float%20%28single-precision%29))
  (bind _wbp_stats_ref (Variables|Default|GetWBP_Stats_Ref))
  (Variables|/Game/UMG/WBP_Stats.WBP_Stats_C|SetSpeedText _wbp_stats_ref (Variables|Default|GetSpeedDisplayString))
  (Variables|/Game/UMG/WBP_Stats.WBP_Stats_C|SetProgressBar%25 _wbp_stats_ref (Variables|Default|GetGasProgress)))

(fn ConstructionScript)